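; BP_Principal is a stealth-game enemy that chases the player and sends them back to a checkpoint with a melee hit.
; Tick runs the chase via AIMoveTo on every branch, so the PawnSensing-driven PlayerVisible flag does not affect it.
; Reaching the player triggers a DoOnce-gated montage whose notify sphere-traces from the right hand.
; A hit loads the checkpoint and clears Hostile; the attack re-arms on montage completion only while Hostile.
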(event OnSeePawn(PawnSensing)
  (params (Pawn :type Pawn%20Object%20Reference))
  (Utilities|Casting|CastToBP_ThirdPersonCharacterCustom Pawn
    (:then
      (Utilities|FlowControl|Sequence
        (:then_0
          (Development|PrintString "Please exit in an calm manner! Stay in line!" true true "(R=0.553125,G=0.000000,B=0.006189,A=1.000000)")
          (Variables|Default|SetbPlayerVisible true))
        (:then_1
          (Utilities|FlowControl|RetriggerableDelay 1.0)
          (Variables|Default|SetbPlayerVisible false))))
    (:CastFailed
      (Variables|Default|SetbPlayerVisible false))))

(event Custom|ChasePlayer
  (CallFunction|UpdateWalkSpeed 6e+02)
  (Variables|Default|SetbCanMove false)
  (AI|AIMoveTo self "0, 0, 0" (Game|GetPlayerCharacter 0) 8e+01 false
    (:OnSuccess
      (CallFunction|Attack))))

(event Custom|Attack
  (bind _mesh (Variables|Character|GetMesh))
  (bind _returnvalue (Transformation|GetSocketLocation _mesh "hand_r"))
  ;[0.15 0.1407 0.04319 0.5] Bonk
  (Utilities|FlowControl|DoOnce false ; Only Reset Attack on miss.
    (:Completed
      (bind _notifyname (Animation|Montage|PlayMontage (Variables|Character|GetMesh) "/Game/StealthGame/Characters/Enemies/AM_Attack_01.AM_Attack_01") ; Play the AM_Attack_01
        (:OnCompleted
          (if (Variables|Default|GetbHostile) ; Keep attacking if you haven't landed the hit.
            (CallFunction|ResetAttack)))
        (:OnNotifyBegin
          (switch name _notifyname ; Pick the proper attack type(standard when there is more than one type of attack)
            (:AttackDamage
              (Development|PrintString "I'm attacking!")
              (bind (_outhits _returnvalue_2) (Collision|MultiSphereTraceForObjects _returnvalue (+ _returnvalue (* (Transformation|GetActorForwardVector) (Variables|Default|GetMeleeTraceDistance))) (Variables|Default|GetMeleeTraceRadius) (Utilities|Array|MakeArray "ObjectTypeQuery3") false 0 "Persistent")) ; Trace forward from hand socket.
              (if _returnvalue_2 ; If a pawn is hit in that trace...
                (for _array_element _outhits ; ...loop through the results....
                  (bind _asbp_third_person_character_custom (Utilities|Casting|CastToBP_ThirdPersonCharacterCustom (.HitActor (Collision|BreakHitResult _array_element))))
                  (Default|LoadCheckpoint _asbp_third_person_character_custom)
                  (Variables|Default|SetbHostile false) ; ...and stop attacking...
                )))))))))

(event Custom|ResetAttack
  (bind _mesh (Variables|Character|GetMesh))
  (bind _returnvalue (Transformation|GetSocketLocation _mesh "hand_r"))
  ;[0.15 0.1407 0.04319 0.5] Bonk
  (Utilities|FlowControl|DoOnce false) ; enters at Reset
)

(event EventBeginPlay
  (Utilities|FlowControl|Sequence
    (:then_0
      (bind _returnvalue (Actor|GetActorOfClass "/Game/StealthGame/Gadgets/NoiseMakers/BP_DistractionItemPawn.BP_DistractionItemPawn_C"))
      (Variables|Default|SetPencilRef _returnvalue))))

(event Collision|EventActorBeginOverlap
  (params (OtherActor :type Actor%20Object%20Reference)))

(event EventTick
  (params (DeltaSeconds :type Float%20%28single-precision%29))
  (if (Variables|Default|GetbCanMove)
    (if (Variables|Default|GetbPlayerVisible)
      (CallFunction|ChasePlayer)
      (else
        (CallFunction|ChasePlayer)))
    (elif (Variables|Default|GetbPlayerVisible)
      (CallFunction|ChasePlayer)
      (else
        (CallFunction|ChasePlayer)))))

(fn ConstructionScript)

(fn UpdateWalkSpeed
  (params (NewWalkSpeed :type Float%20%28double-precision%29))
  (Variables|/Script/Engine.CharacterMovementComponent|SetMaxWalkSpeed (Variables|Character|GetCharacterMovement) NewWalkSpeed))