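; BP_FireAlarm is a stealth-game noise-maker gadget that triggers a one-time fire alarm when the custom player character overlaps its box.
; The overlap passes a DoOnce, then emits AI-audible pawn noise and plays the alarm sound in 2D.
; A sequence then destroys all enemy AI while printing evacuation text, spawns a principal at a fixed transform to chase the player, and destroys all classmates.
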(event OnComponentBeginOverlap(BoxCollision)
  (params (OverlappedComponent :type Primitive%20Component%20Object%20Reference) (OtherActor :type Actor%20Object%20Reference) (OtherComp :type Primitive%20Component%20Object%20Reference) (OtherBodyIndex :type Integer) (bFromSweep :type Boolean) (SweepResult :type Hit%20Result%20Structure%20%28by%20ref%29))
  (Utilities|FlowControl|DoOnce false
    (:Completed
      (Utilities|Casting|CastToBP_ThirdPersonCharacterCustom OtherActor)
      (Class|PawnNoiseEmitterComponent|MakeNoise (Variables|Default|GetPawnNoiseEmitter) self 3.0 (Transformation|GetActorLocation))
      (Audio|PlaySound2D "/Game/StealthGame/Characters/Common/Audio/FireAlarmSFX.FireAlarmSFX" 1.0 1.0 0.0 0 0)
      (Utilities|FlowControl|Sequence
        (:then_0
          (bind _asbp_enemy_ai (Utilities|Casting|CastToBP_EnemyAIClass "/Game/StealthGame/Characters/Enemies/Enemy/BP_EnemyAI.BP_EnemyAI_C"))
          (bind _outactors (Actor|GetAllActorsOfClass _asbp_enemy_ai))
          (for _array_element _outactors
            (Actor|DestroyActor _array_element)
            (Development|PrintString "EVACUATE THE BUILDING" true true "(R=0.278125,G=0.000000,B=0.003112,A=1.000000)") ; This is here instead of in front of for each because I want it to repeat.
          ))
        (:then_1
          (bind _returnvalue (Game|SpawnActorfromClass "/Game/StealthGame/Characters/Enemies/Enemy/BP_Principal.BP_Principal_C" (Math|Transform|MakeTransform "200.000000,-2400.000000,250.000000" "0.000000,90.000000,0.000000" "1.000000,1.000000,1.000000") "Undefined" "MultiplyWithRoot" 0 0))
          (Default|ChasePlayer _returnvalue))
        (:then_2
          (bind _asbp_classmate (Utilities|Casting|CastToBP_ClassmateClass "/Game/StealthGame/Characters/Enemies/Enemy/BP_Classmate.BP_Classmate_C"))
          (bind _outactors_2 (Actor|GetAllActorsOfClass _asbp_classmate))
          (for _array_element_2 _outactors_2
            (Actor|DestroyActor _array_element_2)))))))

(event EventBeginPlay)

(event Collision|EventActorBeginOverlap
  (params (OtherActor :type Actor%20Object%20Reference)))

(event EventTick
  (params (DeltaSeconds :type Float%20%28single-precision%29)))

(fn ConstructionScript)